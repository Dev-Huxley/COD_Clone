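; BP_MainPlayer is the player character Blueprint that handles basic planar movement through Enhanced Input.
; On BeginPlay it adds the IMC_MainPlayer mapping context through the BP_MainPlayerController's local player subsystem.
; IA_MainPlayerMove feeds X to AddMovementYaw and Y to AddMovementPitch, which translate along forward and right vectors despite their names.
; Both offset actor location directly by input times PlayerSpeed, without sweep or delta-time scaling.
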(event `self.ReceiveBeginPlay`
  (bind _asbp_main_player_controller (cast `/Game/MainPlayer/Character/BP_MainPlayerController` (`self.GetController`)))
  (bind _returnvalue (pcsubsystem `EnhancedInputLocalPlayerSubsystem` _asbp_main_player_controller))
  (`/Engine/EditorBlueprintResources/StandardMacros.IsValid` _returnvalue
    (:`Is Valid`
      (`EnhancedInputSubsystemInterface.AddMappingContext` _returnvalue "/Game/MainPlayer/Input/IMC_MainPlayer.IMC_MainPlayer" 0 (struct)))))

(event `EnhancedInput|/Game/MainPlayer/Input/IA_MainPlayerMove`
  (params (ActionValue :type "Vector2D Structure") (ElapsedSeconds :type "Float (double-precision)") (TriggeredSeconds :type "Float (double-precision)") (InputAction :type "InputAction Object Reference" :default "/Game/MainPlayer/Input/IA_MainPlayerMove.IA_MainPlayerMove"))
  (:`Triggered`
    (`self.K2_SetActorLocation` (+ (* (* ActionValue_X (`self.PlayerSpeed`)) (`self.GetActorForwardVector`)) (`self.K2_GetActorLocation`)))
    (`self.K2_SetActorLocation` (+ (* (* ActionValue_Y (`self.PlayerSpeed`)) (`self.GetActorRightVector`)) (`self.K2_GetActorLocation`)))))

(fn `UserConstructionScript`)